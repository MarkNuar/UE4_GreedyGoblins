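; Game mode base for Greedy Goblins that gives each player a random, non-repeating spawn point.
; The construction script caches every PlayerStart actor in the level into an array.
; The ChoosePlayerStart override picks a random entry from that array and removes it before returning it.
; The array is not refilled after picks, and BeginPlay and Tick hold no logic.
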(event `self.ReceiveBeginPlay`)

(fn `ChoosePlayerStart`
  (params (Player :type "Controller Object Reference"))
  (returns (ReturnValue :type "Actor Object Reference"))
  (bind _playerstarts (`self.PlayerStarts`))
  (bind _output_get (set `self.SelectedPlayerStart` (`|GetArrayItem` _playerstarts (`KismetMathLibrary.RandomInteger` (`KismetArrayLibrary.Array_Length` _playerstarts)))))
  (`KismetArrayLibrary.Array_RemoveItem` _playerstarts _output_get)
  (return (`self.SelectedPlayerStart`)))

(fn `UserConstructionScript`
  (bind _outactors (`GameplayStatics.GetAllActorsOfClass` "/Script/Engine.PlayerStart"))
  (set `self.PlayerStarts` _outactors))